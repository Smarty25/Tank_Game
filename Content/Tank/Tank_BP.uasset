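; Player-drivable tank pawn Blueprint that wires its aiming, movement and health bar components together on BeginPlay.
; Input axes drive each track's throttle directly or send forward and turn intent through TankMovement.
; Aim axes rotate an azimuth gimbal and spring arm for the camera, while Fire calls TankAiming.
; The health bar widget receives a reference to this tank.
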(event `self.ReceiveBeginPlay`
  (`TankAimingComponent.Initialize` (`self.TankAiming`) (`self.TankTurret`) (`self.TankBarrel`))
  (`TankMovementComponent.Initialize` (`self.TankMovement`) (`self.TankTrackLeft`) (`self.TankTrackRight`))
  (`self.InitializeHealthBar`))

(event `InputAxis|Track_Left`
  (params (AxisValue :type "Float (single-precision)"))
  (`TankTrack.SetThrottle` (`self.TankTrackLeft`) AxisValue))

(event `InputAxis|Aim_Azimuth`
  (params (AxisValue :type "Float (single-precision)"))
  (`SceneComponent.K2_AddLocalRotation` (`self.Azimuth Gimbal`) (`KismetMathLibrary.MakeRotator` 0.0 0.0 AxisValue) false false))

(event `InputAxis|Track_Right`
  (params (AxisValue :type "Float (single-precision)"))
  (`TankTrack.SetThrottle` (`self.TankTrackRight`) AxisValue))

(event `InputAxis|Aim_Elevation`
  (params (AxisValue :type "Float (single-precision)"))
  (`SceneComponent.K2_AddLocalRotation` (`self.SpringArm`) (`KismetMathLibrary.MakeRotator` 0.0 AxisValue) false false))

(event `InputAxis|IntendMove_Forward/Backward`
  (params (AxisValue :type "Float (single-precision)"))
  (`TankMovementComponent.IntendMoveForward` (`self.TankMovement`) AxisValue))

(event `InputAction|Fire`
  (params (Key :type "Key Structure"))
  (:`Pressed`
    (`TankAimingComponent.Fire` (`self.TankAiming`))))

(event `InputAxis|IntendRotate_Left/Right`
  (params (AxisValue :type "Float (single-precision)"))
  (`TankMovementComponent.IntendTurnRight` (`self.TankMovement`) AxisValue))

(fn `InitializeHealthBar`
  (bind _ashealth_bar (cast `/Game/UI/HealthBar` (`WidgetComponent.GetUserWidgetObject` (`self.HealthBarWidget`))))
  (set `/Game/UI/HealthBar.Tank` self _ashealth_bar))

(fn `UserConstructionScript`)